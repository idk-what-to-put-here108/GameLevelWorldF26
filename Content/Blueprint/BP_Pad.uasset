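; BP_Pad is a healing pad that adds an editable HealthIncrementValue to the player character's health each time an overlap begins.
; Its collision box toggles a healing message, spotlight and hum sound, acting on player 0 without checking which actor overlapped.
; A second collision box shows and hides the points text, which the construction script and BeginPlay set from the increment value.
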(event OnComponentBeginOverlap(CollisionBox)
  (params (OverlappedComponent :type Primitive%20Component%20Object%20Reference) (OtherActor :type Actor%20Object%20Reference) (OtherComp :type Primitive%20Component%20Object%20Reference) (OtherBodyIndex :type Integer) (bFromSweep :type Boolean) (SweepResult :type Hit%20Result%20Structure%20%28by%20ref%29))
  ;[0.15 0.15 0.15 0.5] A good start towards assignement 1
  ;;[0.15 0.15 0.15 0.5] Turns on/off Healiong message when "player" steps on pad
  (Rendering|SetVisibility (Variables|Default|GetTextRender) true false)
  ;;[0.15 0.15 0.15 0.5] Turns light on/off
  (Rendering|Components|Light|SetIntensity (Variables|Default|GetSpotLight) 1.5e+04)
  ;;[0.15 0.15 0.15 0.5] Plays audio, stores a reference to the playing audio, and when needed stops the looping audio
  (bind _returnvalue (Audio|SpawnSound2D "/Game/Audio/hjm-shield_hum_50.hjm-shield_hum_50" 1.0 1.0 0.0 0))
  (Variables|Default|SetPlayingAUdioRef _returnvalue)
  ;[0.15 0.15 0.15 0.5] Adds health based on editable increment value
  (bind _asbp_third_person_character (Utilities|Casting|CastToBP_ThirdPersonCharacter (Game|GetPlayerCharacter 0)))
  (Default|HealthIncrement _asbp_third_person_character (Variables|Default|GetHealthIncrementValue)))

(event OnComponentEndOverlap(CollisionBox)
  (params (OverlappedComponent :type Primitive%20Component%20Object%20Reference) (OtherActor :type Actor%20Object%20Reference) (OtherComp :type Primitive%20Component%20Object%20Reference) (OtherBodyIndex :type Integer))
  ;[0.15 0.15 0.15 0.5] A good start towards assignement 1
  ;;[0.15 0.15 0.15 0.5] Turns on/off Healiong message when "player" steps on pad
  (Rendering|SetVisibility (Variables|Default|GetTextRender) false false)
  ;;[0.15 0.15 0.15 0.5] Turns light on/off
  (Rendering|Components|Light|SetIntensity (Variables|Default|GetSpotLight) 0.0)
  ;;[0.15 0.15 0.15 0.5] Plays audio, stores a reference to the playing audio, and when needed stops the looping audio
  (Audio|Components|Audio|Stop (Variables|Default|GetPlayingAUdioRef)))

(event OnComponentBeginOverlap(CollisionBoxPointsDisplay)
  (params (OverlappedComponent :type Primitive%20Component%20Object%20Reference) (OtherActor :type Actor%20Object%20Reference) (OtherComp :type Primitive%20Component%20Object%20Reference) (OtherBodyIndex :type Integer) (bFromSweep :type Boolean) (SweepResult :type Hit%20Result%20Structure%20%28by%20ref%29))
  ;[0.15 0.15 0.15 0.5] Turn On/Off points display
  (Rendering|SetVisibility (Variables|Default|GetTextRenderPoints) true false))

(event OnComponentEndOverlap(CollisionBoxPointsDisplay)
  (params (OverlappedComponent :type Primitive%20Component%20Object%20Reference) (OtherActor :type Actor%20Object%20Reference) (OtherComp :type Primitive%20Component%20Object%20Reference) (OtherBodyIndex :type Integer))
  ;[0.15 0.15 0.15 0.5] Turn On/Off points display
  (Rendering|SetVisibility (Variables|Default|GetTextRenderPoints) false false))

(event EventBeginPlay
  (Utilities|FlowControl|Sequence
    (:then_0
      ;[0.15 0.15 0.15 0.5] turns off Healing msg
      (Rendering|SetVisibility (Variables|Default|GetTextRender) false false)
      ;[0.15 0.15 0.15 0.5] turns light off
      (Rendering|Components|Light|SetIntensity (Variables|Default|GetSpotLight) 0.0))
    (:then_1
      ;[0.15 0.15 0.15 0.5] Updates render text POINTS
      (Rendering|Components|TextRender|SetText (Variables|Default|GetTextRenderPoints) (Utilities|Text|ToText(Float) (Variables|Default|GetHealthIncrementValue) "HalfToEven")))))

(fn ConstructionScript
  ;[0.15 0.15 0.15 0.5] Updates render text POINTS
  (Rendering|Components|TextRender|SetText (Variables|Default|GetTextRenderPoints) (Utilities|Text|ToText(Float) (Variables|Default|GetHealthIncrementValue) "HalfToEven")))