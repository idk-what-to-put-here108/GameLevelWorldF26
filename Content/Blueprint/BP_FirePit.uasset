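; BP_FirePit is a fire hazard actor that damages actors touching its capsule.
; On BeginPlay, DamageScale sets the particle system's relative scale, so the effect's size tracks its damage.
; Each capsule begin overlap applies BaseDamage times DamageScale to the other actor once, with the pit as damage causer.
; An unconnected leftover branch that directly lowers the third-person character's Health never runs.
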(event OnComponentBeginOverlap(Capsule)
  (params (OverlappedComponent :type Primitive%20Component%20Object%20Reference) (OtherActor :type Actor%20Object%20Reference) (OtherComp :type Primitive%20Component%20Object%20Reference) (OtherBodyIndex :type Integer) (bFromSweep :type Boolean) (SweepResult :type Hit%20Result%20Structure%20%28by%20ref%29))
  (Game|Damage|ApplyDamage OtherActor (* (Variables|Default|GetBaseDamage) (Variables|Default|GetDamageScale)) 0 self))

(event EventBeginPlay
  ;[0.15 0.15 0.15 0.5] Scale size on damage scale
  (Transformation|SetRelativeScale3D (Variables|Default|GetParticleSystem) (Math|Conversions|ToVector(Float) (Variables|Default|GetDamageScale))))

(event Collision|EventActorBeginOverlap
  (params (OtherActor :type Actor%20Object%20Reference)))

(event EventTick
  (params (DeltaSeconds :type Float%20%28single-precision%29)))

(fn ConstructionScript)